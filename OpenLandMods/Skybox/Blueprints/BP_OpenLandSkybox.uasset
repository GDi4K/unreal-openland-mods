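; BP_OpenLandSkybox is a skybox actor that lets each placed instance set its sky texture, rotation, offset and blending with sun and sky atmosphere.
; The construction script creates a dynamic instance of M_OpenLandSkybox on the first material slot of the Skybox component and copies the actor's variables into its parameters.
; The event graph holds only disabled placeholder events, so the Blueprint has no runtime logic.
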(event EventBeginPlay)

(event Collision|EventActorBeginOverlap
  (params (OtherActor :type Actor%20Object%20Reference)))

(event EventTick
  (params (DeltaSeconds :type Float%20%28single-precision%29)))

(fn ConstructionScript
  (bind _returnvalue (Rendering|Material|CreateDynamicMaterialInstance (Variables|Default|GetSkybox) 0 "/Game/OpenLandMods/SkyBox/Materials/M_OpenLandSkybox.M_OpenLandSkybox" "None" :!class /Script/Engine.PrimitiveComponent))
  ;[1 1 1] Set Material Params
  (Rendering|Material|SetTextureParameterValue _returnvalue "Skybox Texture" (Variables|Default|GetSkybox%20Texture))
  (Rendering|Material|SetScalarParameterValue _returnvalue "Skybox Rotation" (Variables|Default|GetSkybox%20Rotation) :!class /Script/Engine.MaterialInstanceDynamic)
  (Rendering|Material|SetVectorParameterValue _returnvalue "Skybox Offset" (Math|Conversions|ToLinearColor(Vector) (Variables|Default|GetSkyBox%20Offset)) :!class /Script/Engine.MaterialInstanceDynamic)
  (Rendering|Material|SetScalarParameterValue _returnvalue "Mix Sun" (Variables|Default|GetMix%20Sun) :!class /Script/Engine.MaterialInstanceDynamic)
  (Rendering|Material|SetScalarParameterValue _returnvalue "Mix Sky Atmosphere" (Variables|Default|GetMix%20Sky%20Atmosphere) :!class /Script/Engine.MaterialInstanceDynamic))